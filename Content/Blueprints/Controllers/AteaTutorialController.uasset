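; Player controller for the Atea VR tutorial, guiding the player through ordered teleport stages and triggering voxel video playback.
; BeginPlay caches the AteaPawn and sorts TutorialTpChecker markers by display name against MarkerList.
; Right trigger on a selectable line-traces for a tag and requests a video, branching on authority.
; Otherwise it aims the teleporter, which only fires if the current marker's thresholds pass, revealing the next, until guidance finishes.
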(event `self.ReceiveBeginPlay`
  ;[1 1 1] If this is called on main menu where AteaController is the default controller, the main menu will randomly disappear
  (`self.SetControlledVrPawn`) ; Assumes VR Only Mode
  (`self.FindAllTpCheckMarkers`))

(event `RequestLoadVoxelVideo`
  (params (TagName :type Name) (MarkerTransform :type "Transform Structure"))
  (`/Game/Blueprints/Actors/VoxelVideoActor.RequestLoadVoxelVideo` (`self.VoxelVideoPlayer`) TagName MarkerTransform))

(event `InputAction|TriggerRight`
  (params (Key :type "Key Structure"))
  (bind _ateapawnref (`self.AteaPawnRef`))
  (bind _ateapawnref_2 (`self.AteaPawnRef`))
  ;[1 1 1] On VoxelVideo Play Selection (Probably not best way to combine)
  (:`Pressed`
    (if (`/Game/Blueprints/Pawns/AteaPawn.OnSelectable` _ateapawnref_2)
      (bind (_tagname _markertransform) (`self.CastSelectionRay` _ateapawnref_2))
      (`/Engine/EditorBlueprintResources/ActorMacros.Switch Has Authority`
        (:`Authority`
          (`/Game/Blueprints/Actors/VoxelVideoActor.RequestLoadVoxelVideo` (`self.VoxelVideoPlayer`) _tagname _markertransform))
        (:`Remote`
          (`self.RequestLoadVoxelVideo` _tagname _markertransform)))
      (else
        (`/Game/Blueprints/Pawns/AteaPawn.ActivateTeleporter` (`self.AteaPawnRef`))
        (`/Game/Blueprints/Actors/TutorialTpChecker.ResetAll` (`|GetArrayItem` (`self.TpCheckMarkers`))))))
  (:`Released`
    (if (`/Game/Blueprints/Pawns/AteaPawn.OnSelectable` _ateapawnref)
      _
      (elif (`self.IsGuidedFinished`)
        (`/Game/Blueprints/Pawns/AteaPawn.Teleport` _ateapawnref)
        (else
          ;;[1 1 1] Guided Tutorial
          (bind _iscorrectpose (`/Game/Blueprints/Actors/TutorialTpChecker.EvaluateThresholds` (`|GetArrayItem` (`self.TpCheckMarkers`) (`self.StageIdx`))))
          (if _iscorrectpose
            (`/Game/Blueprints/Pawns/AteaPawn.Teleport` _ateapawnref)
            (`self.IncrementStage`)
            (`self.RevealNextMarker`)
            (else
              (`/Game/Blueprints/Pawns/AteaPawn.DisableTeleporter` (`self.AteaPawnRef`)))))))))

(event `Key|Escape`
  (params (Key :type "Key Structure"))
  ;[1 1 1] Exit Game
  (:`Pressed`
    (`KismetSystemLibrary.QuitGame` null "Quit")))

(event `CustomEvent_0`
  (params (TagName :type Name) (MarkerActor :type "Actor Object Reference"))
  ;[1 0 0] Results in no owning connection issue
  (`/Game/Blueprints/Actors/VoxelVideoActor.RequestLoadVoxelVideo` (`self.VoxelVideoPlayer`) TagName (`self.GetTransform` MarkerActor)))

(event `UpdateHMDPoseToClients`
  (params (Location :type "Vector Structure") (Rotation :type "Rotator Structure"))
  ;[1 0 0] This does not work as a custom event if your trying to replicate the server HMD pose, there is a conflicting pose updates between client side and server side poses
  (cast `/Game/Blueprints/HMD/VrPawn` (`self.K2_GetPawn`)))

(fn `CastSelectionRay`
  (params (AteaPawn :type "/Game/Blueprints/Pawns/AteaPawn Object Reference"))
  (returns (TagName :type "Name (by ref)") (MarkerTransform :type "Transform Structure"))
  (bind _camera (`/Game/Blueprints/Pawns/AteaPawn.Camera` AteaPawn))
  (bind _right (`/Game/Blueprints/Pawns/AteaPawn.Right` AteaPawn))
  (bind _returnvalue (`SceneComponent.K2_GetComponentLocation` _right))
  (bind _returnvalue_2 (`SceneComponent.K2_GetComponentLocation` _camera))
  (if (`/Game/Blueprints/Pawns/AteaPawn.IsUsingHmd` AteaPawn)
    (bind (_outhit _returnvalue_3) (`KismetSystemLibrary.LineTraceSingle` :`Start` _returnvalue :`End` (+ _returnvalue (* (`KismetMathLibrary.GetForwardVector` (`SceneComponent.K2_GetComponentRotation` _right)) 200.0)) :`TraceChannel` "TraceTypeQuery3" :`DrawTime` 10.0))
    (if _returnvalue_3
      (return (`|GetArrayItem` (`Actor.Tags` (`self.GetAttachParentActor` (`.HitActor` (`GameplayStatics.BreakHitResult` _outhit))))) (`self.GetTransform`)))
    (else
      (bind (_outhit_2 _returnvalue_4) (`KismetSystemLibrary.LineTraceSingle` :`Start` _returnvalue_2 :`End` (+ _returnvalue_2 (* (`KismetMathLibrary.GetForwardVector` (`SceneComponent.K2_GetComponentRotation` _camera)) 200.0)) :`TraceChannel` "TraceTypeQuery3" :`DrawTime` 10.0))
      (if _returnvalue_4
        (return (`|GetArrayItem` (`Actor.Tags` (`self.GetAttachParentActor` (`.HitActor` (`GameplayStatics.BreakHitResult` _outhit_2))))) (`self.GetTransform`))))))

(fn `FindAllTpCheckMarkers`
  (locals (Counter :type Integer) (Size :type Integer) (Idx :type Integer) (TempMarkers :type "Array of /Game/Blueprints/Actors/TutorialTpChecker Object Reference"))
  (bind _outactors (`GameplayStatics.GetAllActorsOfClass` "/Game/Blueprints/Actors/TutorialTpChecker.TutorialTpChecker_C"))
  (set `local.TempMarkers` _outactors)
  (set `local.Size` (`KismetArrayLibrary.Array_Length` _outactors))
  (while (< (`KismetArrayLibrary.Array_Length` (`self.TpCheckMarkers`)) (`local.Size`))
    (if (`KismetStringLibrary.EqualEqual_StrStr` (`|GetArrayItem` (`self.MarkerList`) (`local.Idx`)) (`KismetSystemLibrary.GetDisplayName` (`|GetArrayItem` (`local.TempMarkers`) (`local.Counter`))))
      (`KismetArrayLibrary.Array_Add` (`self.TpCheckMarkers`) (`|GetArrayItem` (`local.TempMarkers`) (`local.Counter`)))
      (`KismetArrayLibrary.Array_Remove` (`local.TempMarkers`) (`local.Counter`))
      (set `local.Counter` 0)
      (`/Engine/EditorBlueprintResources/StandardMacros.IncrementInt` (`local.Idx`))
      (else
        (bind _result (`/Engine/EditorBlueprintResources/StandardMacros.IncrementInt` (`local.Counter`))
          (:`  `
            (if (>= _result (`KismetArrayLibrary.Array_Length` (`local.TempMarkers`)))
              (set `local.Counter` 0)))))))
  (for _array_element (`self.TpCheckMarkers`)
    (`KismetSystemLibrary.PrintString` (`KismetSystemLibrary.GetDisplayName` _array_element))))

(fn `FindVoxelVideoPlayer`
  (bind _outactors (`GameplayStatics.GetAllActorsOfClass` "/Game/Blueprints/Actors/VoxelVideoActor.VoxelVideoActor_C"))
  (set `self.VoxelVideoPlayer` (`|GetArrayItem` _outactors)))

(fn `IncrementStage`
  (if (< (`self.StageIdx`) 16)
    (`/Engine/EditorBlueprintResources/StandardMacros.IncrementInt` (`self.StageIdx`))
    (else
      (set `self.IsGuidedFinished` true))))

(fn `RevealNextMarker`
  (if (`self.IsGuidedFinished`)
    _
    (elif (== (`self.StageIdx`) 0)
      (`SceneComponent.SetVisibility` (`/Game/Blueprints/Actors/TutorialTpChecker.Scene` (`|GetArrayItem` (`self.TpCheckMarkers`) (`self.StageIdx`))) true true)
      (else
        (`SceneComponent.SetVisibility` (`/Game/Blueprints/Actors/TutorialTpChecker.Scene` (`|GetArrayItem` (`self.TpCheckMarkers`) (- (`self.StageIdx`) 1))) false false)
        (`SceneComponent.SetVisibility` (`/Game/Blueprints/Actors/TutorialTpChecker.Scene` (`|GetArrayItem` (`self.TpCheckMarkers`) (`self.StageIdx`))) true true)))))

(fn `SetControlledVrPawn`
  (bind _asatea_pawn (cast `/Game/Blueprints/Pawns/AteaPawn` (`self.K2_GetPawn`)))
  (set `self.AteaPawnRef` _asatea_pawn))

(fn `UserConstructionScript`)