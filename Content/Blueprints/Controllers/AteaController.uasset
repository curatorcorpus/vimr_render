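; AteaController is the player controller for a networked VR app, handling voxel video selection and teleportation.
; On BeginPlay it caches the VR pawn, voxel video player, tagged markers and remote voxel UDP actor, assuming VR-only mode.
; Right trigger either line-traces a selectable to load its tagged video at the matching marker, or teleports the pawn.
; Authority branches update clients directly, while remote branches send requests through controller or pawn events.
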(event `self.ReceiveBeginPlay`
  ;[1 1 1] If this is called on main menu where AteaController is the default controller, the main menu will randomly disappear
  (`self.SetControlledVrPawn`) ; Assumes VR Only Mode
  (`self.FindVoxelVideoPlayer`)
  (`self.GetAllMarkers`)
  (bind _outactors (`GameplayStatics.GetAllActorsWithTag` "RemoteVoxels"))
  (bind _asvoxel_udpactor_replicates (cast `/Game/Blueprints/Actors/VoxelUDPActorReplicates` (`|GetArrayItem` _outactors)))
  (set `self.RemoteVoxelUdpRef` _asvoxel_udpactor_replicates))

(event `RequestLoadVoxelVideo`
  (params (TagName :type Name) (MarkerTransform :type "Transform Structure"))
  (`/Game/Blueprints/Actors/VoxelVideoActor.Multicast_LoadVoxelVideo` (`self.VoxelVideoPlayer`) TagName MarkerTransform))

(event `InputAction|TriggerRight`
  (params (Key :type "Key Structure"))
  (bind _vrpawnref (`self.VrPawnRef`))
  (bind _vrpawnref_2 (`self.VrPawnRef`))
  (bind _rightcontroller (`/Game/Blueprints/HMD/VrPawn.RightController` _vrpawnref_2))
  (bind _rightcontroller_2 (`/Game/Blueprints/HMD/VrPawn.RightController` (`self.VrPawnRef`)))
  ;[1 1 1] On VoxelVideo Play Selection (Probably not best way to combine)
  (:`Pressed`
    (if (`/Game/Blueprints/HMD/CustomBP_MotionController.OnSelectable` _rightcontroller)
      (bind (_tagname _markertransform) (`self.CastSelectionRay` _rightcontroller))
      (`/Engine/EditorBlueprintResources/ActorMacros.Switch Has Authority`
        (:`Authority`
          (`/Game/Blueprints/Actors/VoxelVideoActor.Multicast_LoadVoxelVideo` (`self.VoxelVideoPlayer`) _tagname _markertransform))
        (:`Remote`
          (`self.RequestLoadVoxelVideo` _tagname _markertransform)))
      (else
        (`/Game/Blueprints/HMD/CustomBP_MotionController.ActivateTeleporter` _rightcontroller)
        (`/Engine/EditorBlueprintResources/ActorMacros.Switch Has Authority`
          (:`Authority`
            (`/Game/Blueprints/HMD/VrPawn.ActivateTeleportationMArkerOnClients` _vrpawnref_2))
          (:`Remote`
            (`/Game/Blueprints/HMD/VrPawn.ActivateTeleportationMarkerOnServer` _vrpawnref_2))))))
  (:`Released`
    (if (`/Game/Blueprints/HMD/CustomBP_MotionController.OnSelectable` _rightcontroller_2)
      _
      (elif (`/Game/Blueprints/HMD/CustomBP_MotionController.IsTeleporterActive` _rightcontroller_2)
        (bind (_newlocation _newrotation) (`/Game/Blueprints/HMD/VrPawn.Teleport` _vrpawnref (`/Game/Blueprints/HMD/VrPawn.RightController` _vrpawnref)))
        (`/Engine/EditorBlueprintResources/ActorMacros.Switch Has Authority`
          (:`Authority`
            (`/Game/Blueprints/HMD/VrPawn.UpdateServerVrPoseOnClients` _vrpawnref _newlocation _newrotation)
            (`/Game/Blueprints/HMD/VrPawn.DisableTeleportationMarkerOnClients` _vrpawnref)
            (bind _returnvalue (`KismetMathLibrary.MakeTransform` _newlocation _newrotation))
            (set `/Game/Blueprints/HMD/VrPawn.RemoteTransform` _returnvalue _vrpawnref))
          (:`Remote`
            (`/Game/Blueprints/HMD/VrPawn.UpdateRepVrPoseOnServer` _vrpawnref _newlocation _newrotation)
            (`/Game/Blueprints/HMD/VrPawn.DisableTeleportationMarkerOnServer` _vrpawnref)
            (`/Game/Blueprints/HMD/VrPawn.UpdateRemoteVoxelsOnServer` _vrpawnref _returnvalue)))))))

(event `CustomEvent_0`
  (params (TagName :type Name) (MarkerActor :type "Actor Object Reference"))
  ;[1 0 0] Results in no owning connection issue
  (`/Game/Blueprints/Actors/VoxelVideoActor.RequestLoadVoxelVideo` (`self.VoxelVideoPlayer`) TagName (`self.GetTransform` MarkerActor)))

(event `UpdateHMDPoseToClients`
  (params (Location :type "Vector Structure") (Rotation :type "Rotator Structure"))
  ;[1 0 0] This does not work as a custom event if your trying to replicate the server HMD pose, there is a conflicting pose updates between client side and server side poses
  (cast `/Game/Blueprints/HMD/VrPawn` (`self.K2_GetPawn`)))

(event `Key|Escape`
  (params (Key :type "Key Structure"))
  ;[1 1 1] Exit Game
  (:`Pressed`
    (`KismetSystemLibrary.QuitGame` null "Quit")))

(fn `CastSelectionRay`
  (params (RightController :type "/Game/Blueprints/HMD/CustomBP_MotionController Object Reference"))
  (returns (TagName :type "Name (by ref)") (MarkerTransform :type "Transform Structure"))
  (bind _handmesh (`/Game/Blueprints/HMD/CustomBP_MotionController.HandMesh` RightController))
  (bind _returnvalue (`SceneComponent.K2_GetComponentLocation` _handmesh))
  (bind (_outhit _returnvalue_2) (`KismetSystemLibrary.LineTraceSingle` :`Start` _returnvalue :`End` (+ _returnvalue (* (`KismetMathLibrary.GetForwardVector` (`SceneComponent.K2_GetComponentRotation` _handmesh)) 200.0)) :`TraceChannel` "TraceTypeQuery3" :`DrawDebugType` "ForDuration" :`DrawTime` 10.0))
  (if _returnvalue_2
    (bind _output (`|GetArrayItem` (`Actor.Tags` (`self.GetAttachParentActor` (`.HitActor` (`GameplayStatics.BreakHitResult` _outhit))))))
    (return _output (`self.GetTransform` (`BlueprintMapLibrary.Map_Find` (`self.MarkerActors`) _output)))))

(fn `FindVoxelVideoPlayer`
  (bind _outactors (`GameplayStatics.GetAllActorsOfClass` "/Game/Blueprints/Actors/VoxelVideoActor.VoxelVideoActor_C"))
  (set `self.VoxelVideoPlayer` (`|GetArrayItem` _outactors)))

(fn `GetAllMarkers`
  (bind _outactors (`GameplayStatics.GetAllActorsWithTag` "Marker"))
  (for _array_element _outactors
    (`BlueprintMapLibrary.Map_Add` (`self.MarkerActors`) (`|GetArrayItem` (`Actor.Tags` _array_element)) _array_element)))

(fn `SetControlledVrPawn`
  (bind _asvr_pawn (cast `/Game/Blueprints/HMD/VrPawn` (`self.K2_GetPawn`)))
  (set `self.VrPawnRef` _asvr_pawn))

(fn `UserConstructionScript`)