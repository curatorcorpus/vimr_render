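; Test controller that changes the color of a CubeReplicates actor to exercise networked property changes.
; BeginPlay caches the first CubeReplicates found in the level.
; Space Bar branches on authority: the authority sets the cube's NewColor to a random color directly, while a remote passes one through the RequestColorChange event, which sets the same variable.
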(event `self.ReceiveBeginPlay`
  (bind _outactors (`GameplayStatics.GetAllActorsOfClass` "/Game/Blueprints/CubeReplicates.CubeReplicates_C"))
  (set `self.Cube` (`|GetArrayItem` _outactors)))

(event `Key|SpaceBar`
  (params (Key :type "Key Structure"))
  (bind _returnvalue (`KismetMathLibrary.MakeColor` (`KismetMathLibrary.RandomFloat`) (`KismetMathLibrary.RandomFloat`) (`KismetMathLibrary.RandomFloat`)))
  (:`Pressed`
    (`/Engine/EditorBlueprintResources/ActorMacros.Switch Has Authority`
      (:`Authority`
        (set `/Game/Blueprints/CubeReplicates.NewColor` _returnvalue (`self.Cube`)))
      (:`Remote`
        (`self.RequestColorChange` _returnvalue)))))

(event `RequestColorChange`
  (params (Value :type "LinearColor Structure"))
  (set `/Game/Blueprints/CubeReplicates.NewColor` Value (`self.Cube`)))

(fn `UserConstructionScript`)