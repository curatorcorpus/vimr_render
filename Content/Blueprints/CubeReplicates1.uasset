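; Cube Blueprint that appears to be an unfinished test of replicated colour changes, where the only working behaviour is printing "Hello" on box overlap.
; BeginPlay, the colour-change events and the NewColor OnRep function are all empty.
; Disconnected nodes hold the intended logic: enabling player input, forwarding colour requests, and setting random or replicated colours through dynamic material instances.
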(event `self.ReceiveBeginPlay`)

(event `ChangeColour`)

(event `RequestChangeColor`
  (params (Value :type "LinearColor Structure")))

(event `ChangeAllColor`
  (params (Value :type "LinearColor Structure")))

(event `self.Box.OnComponentBeginOverlap`
  (params (OverlappedComponent :type "PrimitiveComponent Object Reference") (OtherActor :type "Actor Object Reference") (OtherComp :type "PrimitiveComponent Object Reference") (OtherBodyIndex :type Integer) (bFromSweep :type Boolean) (SweepResult :type "HitResult Structure (by ref)"))
  (`KismetSystemLibrary.PrintString` "Hello"))

(fn `OnRep_NewColor`)

(fn `UserConstructionScript`)