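; AteaGameMode is a game mode with debug logging and an editor-only helper for testing in VR or first person.
; BeginPlay on the authority and PostLogin print the name of the player's controlled pawn.
; SelectDefaultPawnEditorOnly skips packaged builds, otherwise spawns and possesses a VrPawn when an HMD is enabled, or a FirstPersonCharacter with its HUD.
; Nothing in this file calls that helper.
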(event `self.ReceiveBeginPlay`
  (`/Engine/EditorBlueprintResources/ActorMacros.Switch Has Authority`
    (:`Authority`
      (`KismetSystemLibrary.PrintString` (`KismetSystemLibrary.GetDisplayName` (`Controller.K2_GetPawn` (`GameplayStatics.GetPlayerController` 0))) true true (struct :`G` 0.66 :`B` 1.0 :`A` 1.0) 20.0))))

(event `self.K2_PostLogin`
  (params (NewPlayer :type "PlayerController Object Reference"))
  (`KismetSystemLibrary.PrintString` (`KismetSystemLibrary.GetDisplayName` (`Controller.K2_GetPawn` NewPlayer)) true true (struct :`G` 0.66 :`B` 1.0 :`A` 1.0) 20.0))

(fn `SelectDefaultPawn (Editor Only)`
  (params (PlayerController :type "PlayerController Object Reference"))
  ;[1 1 1] EDITOR ONLY: This is to switch pawns depending on VR Preview or not in the Editor. Used only for testing.
  (if (`KismetSystemLibrary.IsPackagedForDistribution`)
    (`KismetSystemLibrary.PrintString` "[AteaGameMode Constructor] Not Running Editor Only Code")
    (else
      (`KismetSystemLibrary.PrintString` "Running Editor Only Code" true true (struct :`G` 0.66 :`B` 1.0 :`A` 1.0) 20.0)
      (if (`HeadMountedDisplayFunctionLibrary.IsHeadMountedDisplayEnabled`)
        (`KismetSystemLibrary.PrintString` "USING VR MODE" true true (struct :`G` 0.66 :`B` 1.0 :`A` 1.0) 20.0)
        (bind _returnvalue (`|SpawnActorFromClass` "/Game/Blueprints/HMD/VrPawn.VrPawn_C" (`KismetMathLibrary.MakeTransform` (0.0 0.0 0.0)) "Undefined" "OverrideRootScale" null null))
        (`Controller.Possess` PlayerController _returnvalue)
        (else
          (`KismetSystemLibrary.PrintString` "USING FIRST PERSON MODE" true true (struct :`G` 0.66 :`B` 1.0 :`A` 1.0) 20.0)
          (bind _returnvalue_2 (`|SpawnActorFromClass` "/Game/Blueprints/Characters/FirstPersonCharacter.FirstPersonCharacter_C" (`KismetMathLibrary.MakeTransform` (0.0 0.0 0.0)) "Undefined" "OverrideRootScale" null null))
          (`Controller.Possess` PlayerController _returnvalue_2)
          (`PlayerController.ClientSetHUD` PlayerController "/Game/Blueprints/Widgets/FirstPerson/FirstPersonHUD.FirstPersonHUD_C"))))))

(fn `UserConstructionScript`)