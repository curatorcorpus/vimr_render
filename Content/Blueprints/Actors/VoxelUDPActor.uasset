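; VoxelUDPActor is an actor that renders voxel data from a VoxelUDPSource through its VoxelRender component.
; The construction script assigns the UDP source to the renderer, and collision on the actor is disabled at BeginPlay.
; A Transform function moves the render to a given location and applies only yaw, converted from degrees to a fraction of a turn, as its X rotation.
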(event `self.ReceiveBeginPlay`
  (`self.SetActorEnableCollision` false))

(fn `Transform`
  (params (Location :type "Vector Structure") (Rotation :type "Rotator Structure"))
  (bind _voxelrender (`self.VoxelRender`))
  (`VoxelRenderComponent.SetLocation` _voxelrender Location)
  (`VoxelRenderComponent.SetRotation` _voxelrender (`KismetMathLibrary.MakeVector` (/ (.yaw Rotation) 360.0))))

(fn `UserConstructionScript`
  (set `VoxelRenderComponent.VoxelSource` (`self.VoxelUDPSource`) (`self.VoxelRender`)))