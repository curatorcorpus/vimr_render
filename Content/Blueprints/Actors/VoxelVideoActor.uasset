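; Networked actor that plays voxel video recordings, with audio, positioned at a tagged marker.
; Load requests are relayed through a multicast: a new tag loads the matching .vx3 file, while the current tag toggles play/pause.
; A construction-time link feeds the video source into the voxel renderer, which moves to the marker using only its yaw.
; SelectPlay duplicates the multicast logic locally; actor collision is disabled on BeginPlay.
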(event `self.ReceiveBeginPlay`
  (`self.SetActorEnableCollision` false))

(event `Multicast_LoadVoxelVideo`
  (params (TagName :type Name) (MarkerTransform :type "Transform Structure"))
  ;[0.4475 1 0.5786] Server Multicasts
  (if (== TagName (`self.CurrentTagName`))
    (`self.TogglePlay`)
    (else
      (bind _output_get (set `self.CurrentTagName` TagName))
      (`self.SelectVoxelVideo` _output_get MarkerTransform)
      (set `self.IsPlaying` true))))

(event `RequestLoadVoxelVideo`
  (params (TagName :type Name) (MarkerTransform :type "Transform Structure"))
  ;[1 0.4115 0.4115] Client Requests
  (`self.Multicast_LoadVoxelVideo` TagName MarkerTransform))

(fn `OnRep_CurrentTagName`)

(fn `Pause`
  (`VoxelVideoSourceComponent.Pause` (`self.VoxelVideoSource`)))

(fn `Play`
  (`VoxelVideoSourceComponent.Play` (`self.VoxelVideoSource`)))

(fn `SelectPlay`
  (params (MarkerName :type Name) (MarkerTransform :type "Transform Structure"))
  (if (== MarkerName (`self.CurrentTagName`))
    (`self.TogglePlay`)
    (else
      (bind _output_get (set `self.CurrentTagName` MarkerName))
      (`self.SelectVoxelVideo` _output_get MarkerTransform)
      (set `self.IsPlaying` true))))

(fn `SelectVoxelVideo`
  (params (TagName :type Name) (MarkerTransform :type "Transform Structure"))
  (`VoxelVideoSourceComponent.LoadVoxelVideo` (`self.VoxelVideoSource`) (`KismetStringLibrary.BuildString_Name` "" "" TagName ".vx3"))
  (`self.TransformToMarker` MarkerTransform)
  (`self.Play`))

(fn `Stop`
  (`VoxelVideoSourceComponent.Stop` (`self.VoxelVideoSource`)))

(fn `TogglePlay`
  (bind _voxelvideosource (`self.VoxelVideoSource`))
  (if (`self.IsPlaying`)
    (`VoxelVideoSourceComponent.Pause` _voxelvideosource)
    (set `self.IsPlaying` false)
    (else
      (`VoxelVideoSourceComponent.Play` _voxelvideosource)
      (set `self.IsPlaying` true))))

(fn `TransformToMarker`
  (params (MarkerTransform :type "Transform Structure"))
  (bind _location (.location MarkerTransform))
  (bind _voxelrender (`self.VoxelRender`))
  (`VoxelRenderComponent.SetLocation` _voxelrender _location)
  (`VoxelRenderComponent.SetRotation` _voxelrender (`KismetMathLibrary.MakeVector` (/ (.yaw (.rotation MarkerTransform)) 360.0)))
  (`VoxelVideoSourceComponent.SetAudioLocation` (`self.VoxelVideoSource`) _location))

(fn `UserConstructionScript`
  (set `VoxelRenderComponent.VoxelSource` (`self.VoxelVideoSource`) (`self.VoxelRender`)))