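; Tutorial checker actor, likely for teleports, that measures how an overlapping actor's pose compares with its own.
; Box overlap events store the actor, and each Tick writes its distance and forward-vector dot product to two text components.
; Both texts follow the AteaPawn camera's rotation with a 180-degree local offset.
; SetDebugComponents toggles their visibility from the Debug flag but is not called here, and no pass/fail check exists.
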(event `self.ReceiveTick`
  (params (DeltaSeconds :type "Float (single-precision)"))
  (bind _distancevisualization (`self.DistanceVisualization`))
  (bind _orientationvisualization (`self.OrientationVisualization`))
  (`self.EvaluatePose`)
  (bind _asatea_pawn (cast `/Game/Blueprints/Pawns/AteaPawn` (`Controller.K2_GetPawn` (`GameplayStatics.GetPlayerController` 0))))
  (bind _rotation (.rotation (`SceneComponent.K2_GetComponentToWorld` (`/Game/Blueprints/Pawns/AteaPawn.Camera` _asatea_pawn))))
  (`SceneComponent.K2_SetWorldRotation` _distancevisualization _rotation false false)
  (`SceneComponent.K2_AddLocalRotation` _distancevisualization (struct :`Yaw` 180.0) false false)
  (`SceneComponent.K2_SetWorldRotation` _orientationvisualization _rotation false false)
  (`SceneComponent.K2_AddLocalRotation` _orientationvisualization (struct :`Yaw` 180.0) false false))

(event `self.Box.OnComponentBeginOverlap`
  (params (OverlappedComponent :type "PrimitiveComponent Object Reference") (OtherActor :type "Actor Object Reference") (OtherComp :type "PrimitiveComponent Object Reference") (OtherBodyIndex :type Integer) (bFromSweep :type Boolean) (SweepResult :type "HitResult Structure (by ref)"))
  (set `self.HasOverlappingActor` true)
  (set `self.OtherActor` OtherActor))

(event `self.Box.OnComponentEndOverlap`
  (params (OverlappedComponent :type "PrimitiveComponent Object Reference") (OtherActor :type "Actor Object Reference") (OtherComp :type "PrimitiveComponent Object Reference") (OtherBodyIndex :type Integer))
  (set `self.HasOverlappingActor` false))

(fn `EvaluatePose`
  (bind _otheractor (`self.OtherActor`))
  (if (`self.HasOverlappingActor`)
    (`/Engine/EditorBlueprintResources/StandardMacros.IsValid` _otheractor
      (:`Is Valid`
        (`TextRenderComponent.K2_SetText` (`self.DistanceVisualization`) (`KismetTextLibrary.Conv_StringToText` (`KismetStringLibrary.BuildString_Double` "" "Distance: " (`KismetMathLibrary.VSize` (- (`self.K2_GetActorLocation`) (`self.K2_GetActorLocation` _otheractor))))))
        (`TextRenderComponent.K2_SetText` (`self.OrientationVisualization`) (`KismetTextLibrary.Conv_StringToText` (`KismetStringLibrary.BuildString_Double` "" "Dot: " (`KismetMathLibrary.Dot_VectorVector` (`self.GetActorForwardVector`) (`self.GetActorForwardVector` _otheractor)))))))))

(fn `SetDebugComponents`
  (bind _distancevisualization (`self.DistanceVisualization`))
  (bind _orientationvisualization (`self.OrientationVisualization`))
  (if (`self.Debug`)
    (`SceneComponent.SetVisibility` _distancevisualization true false)
    (`SceneComponent.SetVisibility` _orientationvisualization true false)
    (else
      (`SceneComponent.SetVisibility` _distancevisualization false false)
      (`SceneComponent.SetVisibility` _orientationvisualization false false))))

(fn `UserConstructionScript`)