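; A cube actor Blueprint for changing material colour, with a RepNotify for replicating it.
; ChangeColour applies a random colour, ChangeAllColor applies a passed colour, and OnRep_NewColor applies NewColor, each through a new dynamic material instance.
; RequestChangeColor is empty, nothing here sets NewColor, and the ChangeAllColor call and input enabling are disconnected.
; The Box overlap only prints a debug greeting.
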(event `self.ReceiveBeginPlay`)

(event `ChangeColour`
  (bind _returnvalue (`PrimitiveComponent.CreateDynamicMaterialInstance` (`self.Cube`) 0 "/Game/CubeMaterial_Inst.CubeMaterial_Inst"))
  (`MaterialInstanceDynamic.SetVectorParameterValue` _returnvalue "Color" (`KismetMathLibrary.MakeColor` (`KismetMathLibrary.RandomFloat`) (`KismetMathLibrary.RandomFloat`) (`KismetMathLibrary.RandomFloat`))))

(event `RequestChangeColor`
  (params (Value :type "LinearColor Structure")))

(event `ChangeAllColor`
  (params (Value :type "LinearColor Structure"))
  (bind _returnvalue (`PrimitiveComponent.CreateDynamicMaterialInstance` (`self.Cube`) 0 "/Game/CubeMaterial_Inst.CubeMaterial_Inst"))
  (`MaterialInstanceDynamic.SetVectorParameterValue` _returnvalue "Color" Value))

(event `self.Cube.OnComponentBeginOverlap`
  (params (OverlappedComponent :type "PrimitiveComponent Object Reference") (OtherActor :type "Actor Object Reference") (OtherComp :type "PrimitiveComponent Object Reference") (OtherBodyIndex :type Integer) (bFromSweep :type Boolean) (SweepResult :type "HitResult Structure (by ref)")))

(event `self.Box.OnComponentBeginOverlap`
  (params (OverlappedComponent :type "PrimitiveComponent Object Reference") (OtherActor :type "Actor Object Reference") (OtherComp :type "PrimitiveComponent Object Reference") (OtherBodyIndex :type Integer) (bFromSweep :type Boolean) (SweepResult :type "HitResult Structure (by ref)"))
  (`KismetSystemLibrary.PrintString` "Hello"))

(fn `OnRep_NewColor`
  (bind _returnvalue (`PrimitiveComponent.CreateDynamicMaterialInstance` (`self.Cube`) 0 "/Game/CubeMaterial_Inst.CubeMaterial_Inst"))
  (`MaterialInstanceDynamic.SetVectorParameterValue` _returnvalue "Color" (`self.NewColor`)))

(fn `UserConstructionScript`)