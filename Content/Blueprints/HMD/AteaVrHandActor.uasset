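; AteaVrHandActor is a VR hand actor that shows a Touch controller model for either the left or right hand.
; On BeginPlay it switches on its Hand value to set the MotionController component's motion source to that side.
; Each branch also turns on the component's device model display with a custom source, assigning the matching left or right Touch controller mesh.
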(event `self.ReceiveBeginPlay`
  (bind _motioncontroller (`self.MotionController`))
  (bind _motioncontroller_2 (`self.MotionController`))
  (switch `EControllerHand` (`self.Hand`)
    (:`Left`
      (set `MotionControllerComponent.MotionSource` "Left" _motioncontroller_2)
      (set `MotionControllerComponent.bDisplayDeviceModel` true _motioncontroller_2)
      (set `MotionControllerComponent.DisplayModelSource` "Custom" _motioncontroller_2)
      (set `MotionControllerComponent.CustomDisplayMesh` "/Game/TexturedModels/Meshes/Oculus/LeftTouchController.LeftTouchController" _motioncontroller_2))
    (:`Right`
      (set `MotionControllerComponent.MotionSource` "Right" _motioncontroller)
      (set `MotionControllerComponent.bDisplayDeviceModel` true _motioncontroller)
      (set `MotionControllerComponent.DisplayModelSource` "Custom" _motioncontroller)
      (set `MotionControllerComponent.CustomDisplayMesh` "/Game/TexturedModels/Meshes/Oculus/RightTouchController.RightTouchController" _motioncontroller))))

(fn `UserConstructionScript`)